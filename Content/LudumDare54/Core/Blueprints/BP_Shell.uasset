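; BP_Shell is a shell actor for a Ludum Dare 54 game that randomizes its appearance on spawn.
; BeginPlay sets a random mesh from Meshes, then picks a random color material from the set selected by the Random node's index.
; That pure node re-evaluates for the material call, so mesh and material set can mismatch.
; The construction script sizes interaction and collision spheres from base radii; InteractBP is empty.
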(event EventBeginPlay
  (bind _meshes (Variables|Default|GetMeshes))
  (bind _shellmesh (Variables|Default|GetShellMesh))
  (bind (_outitem _outindex) (Utilities|Array|Random _meshes))
  (Components|StaticMesh|SetStaticMesh _shellmesh _outitem)
  (Rendering|Material|SetMaterial _shellmesh 0 (Utilities|Select :Index _outindex :Option%200 (Utilities|Select :Index (Math|Random|RandomIntegerinRange 0 1) :Option%200 "/Game/LudumDare54/Art/Materials/Shell1/M_Shell1_Blue.M_Shell1_Blue" :Option%201 "/Game/LudumDare54/Art/Materials/Shell1/M_Shell1_Orange.M_Shell1_Orange") :Option%201 (Utilities|Select :Index (Math|Random|RandomIntegerinRange 0 2) :Option%200 "/Game/LudumDare54/Art/Materials/Shell2/M_Shell2_Green.M_Shell2_Green" :Option%201 "/Game/LudumDare54/Art/Materials/Shell2/M_Shell2_Pink.M_Shell2_Pink" :Option%202 "/Game/LudumDare54/Art/Materials/Shell2/M_Shell2_Yellow.M_Shell2_Yellow"))))

(event Collision|EventActorBeginOverlap
  (params (OtherActor :type Actor%20Object%20Reference)))

(event EventTick
  (params (DeltaSeconds :type Float%20%28single-precision%29)))

(event EventInteractBP
  (params (Instigator :type Actor%20Object%20Reference)))

(fn ConstructionScript
  (Components|Sphere|SetSphereRadius (Variables|Default|GetInteract%20Sphere) (Variables|Default|GetBaseInteractRadius) true)
  (Components|Sphere|SetSphereRadius (Variables|Default|GetCollisionSphere) (Variables|Default|GetBaseCollisionRadius) true))