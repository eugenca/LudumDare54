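; BP_HermitPlayer is the hermit player character, which detects shells within reach and prompts the player to equip one.
; InteractSphere overlap events maintain a list of reachable BP_Shell actors.
; Each Tick picks the closest as NearestShell and toggles the equip tip on the player controller's HUD widget.
; The construction script sizes the sphere and capsule from base radii and lowers the mesh to the capsule's bottom.
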(event Custom|CustomEvent
  (params (OverlappedComponent :type Primitive%20Component%20Object%20Reference) (OtherActor :type Actor%20Object%20Reference) (OtherComp :type Primitive%20Component%20Object%20Reference) (OtherBodyIndex :type Integer) (bFromSweep :type Boolean) (SweepResult :type Hit%20Result%20Structure%20%28by%20ref%29))
  (bind _asbp_shell (Utilities|Casting|CastToBP_Shell OtherActor))
  (Utilities|Array|AddUnique (Variables|Default|GetReachableShells) _asbp_shell))

(event Custom|OnComponentEndOverlap_Event
  (params (OverlappedComponent :type Primitive%20Component%20Object%20Reference) (OtherActor :type Actor%20Object%20Reference) (OtherComp :type Primitive%20Component%20Object%20Reference) (OtherBodyIndex :type Integer))
  (bind _asbp_shell (Utilities|Casting|CastToBP_Shell OtherActor))
  (Utilities|Array|RemoveItem (Variables|Default|GetReachableShells) _asbp_shell))

(event EventBeginPlay
  (Collision|BindEventtoOnComponentBeginOverlap (Variables|Default|GetInteractSphere) (delegate Custom|CustomEvent))
  (Collision|AssignOnComponentEndOverlap (Variables|Default|GetInteractSphere) (delegate Custom|OnComponentEndOverlap_Event)))

(event Collision|EventActorBeginOverlap
  (params (OtherActor :type Actor%20Object%20Reference)))

(event EventTick
  (params (DeltaSeconds :type Float%20%28single-precision%29))
  (Variables|Default|SetNearestShell 0)
  (Variables|Default|SetMinDist 9999.0)
  (for _array_element (Variables|Default|GetReachableShells)
    (if (< (Math|Vector|Distance(Vector) (Transformation|GetActorLocation) (Transformation|GetActorLocation _array_element)) (Variables|Default|GetMinDist))
      (Variables|Default|SetMinDist (Math|Vector|Distance(Vector) (Transformation|GetActorLocation) (Transformation|GetActorLocation _array_element)))
      (Variables|Default|SetNearestShell _array_element)))
  (bind _asbp_hermit_player_controller (Utilities|Casting|CastToBP_HermitPlayerController (Game|GetPlayerController 0)))
  (Default|ToggleEquipShellTip (Variables|/Game/LudumDare54/Core/Blueprints/BP_HermitPlayerController.BP_HermitPlayerController_C|GetHudWidget _asbp_hermit_player_controller) (Utilities|IsValid (Variables|Default|GetNearestShell))))

(fn ConstructionScript
  (bind _basecollisionradius (Variables|Default|GetBaseCollisionRadius))
  (Components|Sphere|SetSphereRadius (Variables|Default|GetInteractSphere) (Variables|Default|GetBaseInteractRadius) true)
  (Components|Capsule|SetCapsuleSize (Variables|Default|GetCapsuleComponent) _basecollisionradius _basecollisionradius true)
  (Transformation|SetRelativeLocation (Variables|Character|GetMesh) (+ "" (Math|Vector|MakeVector 0.0 0.0 (- 0.0 (Variables|Default|GetBaseCollisionRadius)))) false false))