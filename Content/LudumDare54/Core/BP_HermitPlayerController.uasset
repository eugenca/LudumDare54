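; Player controller for the Ludum Dare 54 hermit game that switches the on-screen UI with the gameplay state.
; On BeginPlay it binds to the game mode's state-change event, creates collapsed main menu, HUD and end-game widgets, then starts in the main menu state.
; Each state change collapses the current widget and shows the mapped one, with ScoreTable and End reusing the main menu.
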(event Custom|OnGameplayStateChanged_Event
  (params (NewState :type EHermitGameplayState%20Enum :default "MainMenu") (OldState :type EHermitGameplayState%20Enum :default "MainMenu"))
  (bind _mainmenuwidget (Variables|Default|GetMainMenuWidget))
  (Widget|SetVisibility (Variables|Default|GetCurrentWidgetRef) "Collapsed")
  (bind _output_get (Variables|Default|SetCurrentWidgetRef (Utilities|Select :Index NewState :MainMenu _mainmenuwidget :PlayingCharacter (Variables|Default|GetHudWidget) :EndGameSequence (Variables|Default|GetEndGameWidget) :ScoreTable _mainmenuwidget :End _mainmenuwidget)))
  (Widget|SetVisibility _output_get "Visible"))

(event EventBeginPlay
  (bind _asludum_54gm (Utilities|Casting|CastToLudum54GM (Game|GetGameMode)))
  (EventDispatchers|AssignOnGameplayStateChanged _asludum_54gm (delegate Custom|OnGameplayStateChanged_Event))
  (Utilities|FlowControl|Sequence
    (:then_0
      (bind _returnvalue (UserInterface|CreateWidget "/Game/LudumDare54/Core/UI/W_MainMenu.W_MainMenu_C"))
      (bind _output_get (Variables|Default|SetMainMenuWidget _returnvalue))
      (UserInterface|Viewport|AddtoViewport _output_get 0)
      (Widget|SetVisibility _output_get "Collapsed")
      (Variables|Default|SetCurrentWidgetRef _output_get))
    (:then_1
      (bind _returnvalue_2 (UserInterface|CreateWidget "/Game/LudumDare54/Core/UI/W_HUD.W_HUD_C"))
      (bind _output_get_2 (Variables|Default|SetHudWidget _returnvalue_2))
      (UserInterface|Viewport|AddtoViewport _output_get_2 0)
      (Widget|SetVisibility _output_get_2 "Collapsed"))
    (:then_2
      (bind _returnvalue_3 (UserInterface|CreateWidget "/Game/LudumDare54/Core/UI/W_EndGameWidget.W_EndGameWidget_C"))
      (bind _output_get_3 (Variables|Default|SetEndGameWidget _returnvalue_3))
      (UserInterface|Viewport|AddtoViewport _output_get_3 0)
      (Widget|SetVisibility _output_get_3 "Collapsed"))
    (:then_3
      (CallFunction|OnGameplayStateChangedEvent "MainMenu" "MainMenu"))))

(event EventTick
  (params (DeltaSeconds :type Float%20%28single-precision%29)))

(fn ConstructionScript)

(fn SetWidgetVisibility
  (params (bVisible :type Boolean))
  (Widget|SetVisibility (Variables|Default|GetMainMenuWidget) (select bVisible "Visible" "Collapsed")))